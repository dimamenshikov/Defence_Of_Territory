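; Player character that spawns a difficulty-scaled rifle on its spine and ends the game as lost when fewer than two defence blocks remain.
; Shoot mode uses equip montage notifies, played forward or reversed, to move the rifle between hand and spine and toggle gameplay abilities, also clearing crouch on exit.
; Also registers itself in GameplayClasses, switches spring-arm framing for camera focus and enables ragdoll on death.
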(event `self.ReceiveBeginPlay`
  ;[0 0 0] Запись себя в геймплейный класс, создание и крепление оружия к себе, подписка на уничтожение объектов
  (`parent.ReceiveBeginPlay`)
  (set `/Game/TestSkillbox/Blueprint/DataAsset/PDA_GameplayClasses.TestSkillbox_P` self (`self.GameplayClasses`))
  (bind _returnvalue (`|SpawnActorFromClass` "/Game/TestSkillbox/Blueprint/Environment/Weapon/BP_Rifle.BP_Rifle_C" (`KismetMathLibrary.MakeTransform` (0.0 0.0 0.0)) "Undefined" "MultiplyWithRoot" null (select `/Game/TestSkillbox/Blueprint/Enum/E_GameDifficulty` (`/Game/TestSkillbox/Core/BP_TestSkillbox_GI.GameDifficulty` (`/Game/TestSkillbox/Blueprint/DataAsset/PDA_GameplayClasses.TestSkillbox_GI` (`self.GameplayClasses`))) :`NewEnumerator0` 600 :`NewEnumerator1` 400 :`NewEnumerator2` 200) self null))
  (bind _output_get (set `self.ActiveWeapon` _returnvalue))
  (`self.K2_AttachToComponent` _output_get (`self.Spine`) "None" "KeepRelative" "KeepRelative" "KeepRelative" true)
  (`self.K2_SetActorRelativeTransform` (`self.ActiveWeapon`) (`KismetMathLibrary.MakeTransform` (0.0 0.0 0.0)) false false)
  (bind _outactors (`GameplayStatics.GetAllActorsOfClass` "/Game/TestSkillbox/Blueprint/Environment/BP_DefenceBlock.BP_DefenceBlock_C"))
  (bind _output_get_2 (set `self.DefencesObject` _outactors))
  (for _array_element _output_get_2
    (add `self.OnDestroyed` _array_element (delegate `DefencesObjectDestroy`))))

(event `DefencesObjectDestroy` :!signature `self.OnDestroyed`
  (params (DestroyedActor :type "Actor Object Reference"))
  (bind _defencesobject (`self.DefencesObject`))
  (bind _numerobject (`self.NumerObject`))
  ;[0 0 0] Запись себя в геймплейный класс, создание и крепление оружия к себе, подписка на уничтожение объектов
  (set `self.NumerObject` -1)
  (for (_array_element _array_index) (`self.DefencesObject`)
    (if (== DestroyedActor _array_element)
      (set `self.NumerObject` _array_index)
      (break)))
  (if (!= _numerobject -1)
    (`KismetArrayLibrary.Array_RemoveItem` (`self.DefencesObject`) (`|GetArrayItem` _defencesobject _numerobject))
    (if (< (`KismetArrayLibrary.Array_Length` _defencesobject) 2)
      (`/Game/TestSkillbox/Core/BP_TestSkillBox_GM.EndGame` (`/Game/TestSkillbox/Blueprint/DataAsset/PDA_GameplayClasses.TestSkillbox_GM` (`self.GameplayClasses`)) false))))

(event `Death`
  ;[0 0 0] Включение Ragdoll
  (`self.Ragdoll` true))

(event `FocusCamera`
  (params (FocusCamera :type Boolean))
  (bind _springarm (`self.SpringArm`))
  ;[0 0 0] Приближение/отдаление камеры к персонажу
  (set `SpringArmComponent.SocketOffset` (`KismetMathLibrary.SelectVector` (0.0 40.0 60.0) (0.0 100.0 60.0) FocusCamera) _springarm)
  (set `SpringArmComponent.TargetArmLength` (`KismetMathLibrary.SelectFloat` 30.0 300.0 FocusCamera) _springarm))

(event `ModeShoot`
  (params (ModeShoot :type Boolean))
  (bind _activeweapon (`self.ActiveWeapon`))
  ;[0 0 0] Режим стрельбы
  (`self.ActiveWeapon`
    (:`then`
      (if (not (`NavMovementComponent.IsFalling` (`self.CharacterMovement`)))
        (set `self.Mode Shoot` true)
        (if ModeShoot
          (`|ExecutionSequence`
            (:`then_0`
              (goto _label :!via `Open`))
            (:`then_1`
              (`|PlayMontage` (`self.Mesh`) "/Game/TestSkillbox/Animation/MannyASP/AM_Equip_Rifle.AM_Equip_Rifle"
                (:`OnNotifyBegin`
                  (`/Engine/EditorBlueprintResources/StandardMacros.Gate` true :!label _label
                    (:`Exit`
                      (`|ExecutionSequence`
                        (:`then_0`
                          (`/Engine/EditorBlueprintResources/StandardMacros.FlipFlop`
                            (:`A`
                              (`self.K2_AttachToComponent` _activeweapon (`self.Hand`) "None" "KeepRelative" "KeepRelative" "KeepRelative" true)
                              (`self.K2_SetActorRelativeTransform` _activeweapon (`KismetMathLibrary.MakeTransform` (0.0 0.0 0.0)) false false))
                            (:`B`
                              (`self.ActiveAbility` true "/Game/TestSkillbox/Blueprint/AbilitySystem/GA_ModeShoot.GA_ModeShoot_C")
                              (set `self.Mode Shoot` false))))
                        (:`then_1`
                          (goto _label_2 :!via `Reset`)))))))))
          (else
            (`|ExecutionSequence`
              (:`then_0`
                (goto _label :!via `Close`))
              (:`then_1`
                (`|PlayMontage` (`self.Mesh`) "/Game/TestSkillbox/Animation/MannyASP/AM_Equip_Rifle.AM_Equip_Rifle" -1.0 1.13
                  (:`then`
                    (`self.ActiveAbility` false "/Game/TestSkillbox/Blueprint/AbilitySystem/GA_ModeShoot.GA_ModeShoot_C")
                    (if (`BlueprintGameplayTagLibrary.HasTag` (`GameplayTagAssetInterface.GetOwnedGameplayTags` (`self.AbilitySystem`)) (struct :`TagName` "Status.Character.Crouch"))
                      (`self.ActiveAbility` false "/Game/TestSkillbox/Blueprint/AbilitySystem/GA_Crouch.GA_Crouch_C")
                      (`SceneComponent.K2_SetRelativeLocation` (`self.SpringArm`) (0.0 50.0 40.0) false false)))
                  (:`OnNotifyBegin`
                    (`/Engine/EditorBlueprintResources/StandardMacros.DoOnce` true :!label _label_2
                      (:`Completed`
                        (`KismetSystemLibrary.Delay` 0.5)
                        (`self.K2_AttachToComponent` (`self.ActiveWeapon`) (`self.Spine`) "None" "KeepRelative" "KeepRelative" "KeepRelative" true)
                        (`self.K2_SetActorRelativeTransform` (`self.ActiveWeapon`) (`KismetMathLibrary.MakeTransform` (0.0 0.0 0.0)) false false)
                        (set `self.Mode Shoot` false)))))))))))
    (:`else`)))

(fn `UserConstructionScript`)