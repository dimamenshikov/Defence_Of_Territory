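; Player state Blueprint for TestSkillbox that tracks the player's best completion time.
; On BeginPlay it registers itself in the shared GameplayClasses references and copies the record from the game instance.
; EndGame updates and saves the record through the game instance when a win beats it or none exists.
; ClearRecord zeroes both copies and deletes the save slot.
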(event `self.ReceiveBeginPlay`
  (bind _gameplayclasses (`self.GameplayClasses`))
  ;[0 0 0] Запись себя в геймплейный класс, запись рекорда
  (set `/Game/TestSkillbox/Blueprint/DataAsset/PDA_GameplayClasses.TestSkillbox_PS` self _gameplayclasses)
  (set `self.Record` (`/Game/TestSkillbox/Core/BP_TestSkillbox_GI.Record` (`/Game/TestSkillbox/Blueprint/DataAsset/PDA_GameplayClasses.TestSkillbox_GI` _gameplayclasses))))

(fn `ClearRecord`
  (bind _testskillbox_gi (`/Game/TestSkillbox/Blueprint/DataAsset/PDA_GameplayClasses.TestSkillbox_GI` (`self.GameplayClasses`)))
  ;[0 0 0] Удаление сохранённого рекорда
  (set `self.Record` 0.0)
  (set `/Game/TestSkillbox/Core/BP_TestSkillbox_GI.Record` 0.0 _testskillbox_gi)
  (`GameplayStatics.DeleteGameInSlot` (`/Game/TestSkillbox/Core/BP_TestSkillbox_GI.Slot Name` _testskillbox_gi)))

(fn `EndGame`
  (params (Win :type Boolean) (Time :type "Float (double-precision)"))
  (bind _record (`self.Record`))
  (bind _testskillbox_gi (`/Game/TestSkillbox/Blueprint/DataAsset/PDA_GameplayClasses.TestSkillbox_GI` (`self.GameplayClasses`)))
  ;[0 0 0] Сохранение рекорда при победе
  (if (and Win (or (< Time _record) (== _record 0.0)))
    (bind _output_get (set `self.Record` Time))
    (bind _output_get_2 (set `/Game/TestSkillbox/Core/BP_TestSkillbox_GI.Record` _output_get _testskillbox_gi))
    (`/Game/TestSkillbox/Core/BP_TestSkillbox_GI.SaveRecord` _testskillbox_gi _output_get_2)))

(fn `UserConstructionScript`)