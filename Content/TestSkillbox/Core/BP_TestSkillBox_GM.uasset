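; Game mode for TestSkillbox that runs the match flow: delayed start, game timer, win or defeat, and pause.
; It registers itself in a shared GameplayClasses reference, starts a looping timer that broadcasts elapsed time, and binds to the player's death for defeat.
; Ending passes the result and time to the player state, toggles pause, updates the HUD and plays a result sound.
; Level music volume follows game instance settings, and pausing switches input mode and cursor.
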(event `self.ReceiveBeginPlay`
  (bind (_gamesetting_sound _gamesetting_music _gamesetting_audio) (break `/Game/TestSkillbox/Blueprint/Structure/S_GameSetting` (`/Game/TestSkillbox/Core/BP_TestSkillbox_GI.GameSetting` (`/Game/TestSkillbox/Blueprint/DataAsset/PDA_GameplayClasses.TestSkillbox_GI` (`self.GameplayClasses`)))))
  ;[0 0 0] Запись себя в геймплейный класс, подписка на изменение настроек игры, старт игры
  (set `/Game/TestSkillbox/Blueprint/DataAsset/PDA_GameplayClasses.TestSkillbox_GM` self (`self.GameplayClasses`))
  (`AudioComponent.SetVolumeMultiplier` (`self.LevelMusic`) (* _gamesetting_music _gamesetting_audio))
  (add `/Game/TestSkillbox/Core/BP_TestSkillbox_GI.OnChangeGameSetting` (`/Game/TestSkillbox/Blueprint/DataAsset/PDA_GameplayClasses.TestSkillbox_GI` (`self.GameplayClasses`)) (`|CreateDelegate` :!event `ChangeGameSetting`))
  (`KismetSystemLibrary.Delay` 0.5)
  (`self.StartGame`))

(event `StartGame`
  ;[0 0 0] Старт игры, запуск секундомера игры
  (`self.OnStartGame`)
  (bind _returnvalue (`KismetSystemLibrary.K2_SetTimerDelegate` (`|CreateDelegate` :!event `UpdateTime Game`) 0.1 true))
  (set `self.TimeGame` _returnvalue)
  (add `/Game/TestSkillbox/Blueprint/Character/BP_BaseCharacter.OnDeath` (`/Game/TestSkillbox/Blueprint/DataAsset/PDA_GameplayClasses.TestSkillbox_P` (`self.GameplayClasses`)) (`|CreateDelegate` :!event `PlayerDeath`)))

(event `EndGame`
  (params (Win :type Boolean :default true))
  (bind _gameplayclasses (`self.GameplayClasses`))
  (bind _win (`self.Win`))
  (bind (_gamesetting_sound _gamesetting_music _gamesetting_audio) (break `/Game/TestSkillbox/Blueprint/Structure/S_GameSetting` (`/Game/TestSkillbox/Core/BP_TestSkillbox_GI.GameSetting` (`/Game/TestSkillbox/Blueprint/DataAsset/PDA_GameplayClasses.TestSkillbox_GI` (`self.GameplayClasses`)))))
  ;[0 0 0] Конец игры, запись рекордного времени
  (set `self.Win` Win)
  (`KismetSystemLibrary.Delay` 2.0)
  (`KismetSystemLibrary.K2_ClearAndInvalidateTimerHandle` (`self.TimeGame`))
  (`/Game/TestSkillbox/Core/BP_TestSkillbox_PS.EndGame` (`/Game/TestSkillbox/Blueprint/DataAsset/PDA_GameplayClasses.TestSkillbox_PS` _gameplayclasses) (`self.Win`) (`self.Time`))
  (`self.SetGamePause` false)
  (`/Game/TestSkillbox/Core/BP_TestSkillbox_HUD.EndGame` (`/Game/TestSkillbox/Blueprint/DataAsset/PDA_GameplayClasses.TestSkillbox_HUD` _gameplayclasses) _win)
  (`GameplayStatics.PlaySound2D` (select `bool` _win :`false` "/Game/TestSkillbox/Assets/Audio/A_Defeat.A_Defeat" :`true` "/Game/TestSkillbox/Assets/Audio/A_Win.A_Win" :!type "SoundBase Object Reference") (* _gamesetting_music _gamesetting_audio) 1.0 0.0 null null))

(event `PlayerDeath`
  ;[0 0 0] Поражение
  (`KismetSystemLibrary.Delay` 3.0)
  (`self.EndGame` false))

(event `ChangeGameSetting`
  (params (GameSetting :type "/Game/TestSkillbox/Blueprint/Structure/S_GameSetting Structure"))
  ;[0 0 0] Изменение громкости музыки
  (`AudioComponent.SetVolumeMultiplier` (`self.LevelMusic`) (* GameSetting_Music_8_F5472D50425BD29401330E9AC43CA930 GameSetting_Audio_9_7DE9B5BF488BD0CA4371A8A2225B1AD7)))

(fn `SetGamePause`
  (params (HUD_Pause :type Boolean :default true))
  (bind _returnvalue (`GameplayStatics.IsGamePaused`))
  ;[0 0 0] Пауза/продолжение игры
  (`GameplayStatics.SetGamePaused` (not _returnvalue))
  (`self.SetInputMode` (select `bool` _returnvalue :`false` "NewEnumerator2" :`true` "NewEnumerator1" :!type "/Game/TestSkillbox/Blueprint/Enum/E_InputMode Enum"))
  (if HUD_Pause
    (`/Game/TestSkillbox/Core/BP_TestSkillbox_HUD.PauseGame` (`/Game/TestSkillbox/Blueprint/DataAsset/PDA_GameplayClasses.TestSkillbox_HUD` (`self.GameplayClasses`)) (`GameplayStatics.IsGamePaused`))))

(fn `SetInputMode`
  (params (InputMode :type "/Game/TestSkillbox/Blueprint/Enum/E_InputMode Enum" :default "NewEnumerator0"))
  (bind _testskillbox_pc (`/Game/TestSkillbox/Blueprint/DataAsset/PDA_GameplayClasses.TestSkillbox_PC` (`self.GameplayClasses`)))
  (bind _testskillbox_pc_2 (`/Game/TestSkillbox/Blueprint/DataAsset/PDA_GameplayClasses.TestSkillbox_PC` (`self.GameplayClasses`)))
  ;[0 0 0] Установка режима ввода контроллера
  (switch `/Game/TestSkillbox/Blueprint/Enum/E_InputMode` InputMode
    (:`NewEnumerator0`
      (`WidgetBlueprintLibrary.SetInputMode_UIOnlyEx` _testskillbox_pc null "DoNotLock" true)
      (set `PlayerController.bShowMouseCursor` true _testskillbox_pc_2 :!label _label))
    (:`NewEnumerator1`
      (`WidgetBlueprintLibrary.SetInputMode_GameAndUIEx` _testskillbox_pc null)
      (goto _label))
    (:`NewEnumerator2`
      (`WidgetBlueprintLibrary.SetInputMode_GameOnly` _testskillbox_pc)
      (set `PlayerController.bShowMouseCursor` false _testskillbox_pc_2))))

(fn `UpdateTime Game`
  ;[0 0 0] Обновление времени игры
  (bind _output_get (set `self.Time` (+ (`self.Time`) 0.1)))
  (`self.OnUpdateTimeGame` _output_get))

(fn `UserConstructionScript`)