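; Menu game mode that starts the main menu screen and keeps the level music volume in line with game settings.
; On BeginPlay it sets LevelMusic volume to Music times Audio from the game instance settings, then shows WBP_MainMenu with mouse cursor and UI-only input.
; It also binds to the game instance's OnChangeGameSetting dispatcher to update the music volume when settings change.
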(event `self.ReceiveBeginPlay`
  (bind _returnvalue (`GameplayStatics.GetPlayerController` 0))
  (bind (_gamesetting_sound _gamesetting_music _gamesetting_audio) (break `/Game/TestSkillbox/Blueprint/Structure/S_GameSetting` (`/Game/TestSkillbox/Core/BP_TestSkillbox_GI.GameSetting` (`/Game/TestSkillbox/Blueprint/DataAsset/PDA_GameplayClasses.TestSkillbox_GI` (`self.GameplayClasses`)))))
  ;[0 0 0] Включение музыки, показ главного меню, подписка на изменение настроек игры
  (`AudioComponent.SetVolumeMultiplier` (`self.LevelMusic`) (* _gamesetting_music _gamesetting_audio))
  (bind _returnvalue_2 (`|CreateWidget` "/Game/TestSkillbox/Widget/WBP_MainMenu.WBP_MainMenu_C"))
  (`UserWidget.AddToViewport` _returnvalue_2 0)
  (set `PlayerController.bShowMouseCursor` true _returnvalue)
  (`WidgetBlueprintLibrary.SetInputMode_UIOnlyEx` _returnvalue null)
  (add `/Game/TestSkillbox/Core/BP_TestSkillbox_GI.OnChangeGameSetting` (`/Game/TestSkillbox/Blueprint/DataAsset/PDA_GameplayClasses.TestSkillbox_GI` (`self.GameplayClasses`)) (`|CreateDelegate` :!event `ChangeVolumeMusic`)))

(event `ChangeVolumeMusic`
  (params (NewParam :type "/Game/TestSkillbox/Blueprint/Structure/S_GameSetting Structure"))
  ;[0 0 0] Изменение громкости музыки
  (`AudioComponent.SetVolumeMultiplier` (`self.LevelMusic`) (* NewParam_Music_8_F5472D50425BD29401330E9AC43CA930 NewParam_Audio_9_7DE9B5BF488BD0CA4371A8A2225B1AD7)))

(fn `UserConstructionScript`)