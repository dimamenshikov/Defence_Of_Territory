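; Player controller that registers itself in GameplayClasses, adds the Enhanced Input mapping and routes input to the pawn, HUD and game mode.
; Movement and look apply directly, while actions such as jump, sprint, crouch, fix, reload, shoot and aim trigger pawn gameplay abilities.
; Gates loop fire while held and separate aim taps, which toggle shoot mode, from delayed holds that activate aiming.
; Gameplay tags drive crouch toggling and aim-state checks.
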(event `self.ReceiveBeginPlay`
  ;[0 0 0] Запись себя в геймплейный класс, подключение системы привязки клавиш
  (set `/Game/TestSkillbox/Blueprint/DataAsset/PDA_GameplayClasses.TestSkillbox_PC` self (`self.GameplayClasses`))
  (`EnhancedInputSubsystemInterface.AddMappingContext` (subsystem `EnhancedInputLocalPlayerSubsystem`) "/Game/TestSkillbox/Input/IMC_Management.IMC_Management" 0 (struct))
  (`WidgetBlueprintLibrary.SetInputMode_GameOnly` self true)
  (set `self.bShowMouseCursor` false))

(event `EnhancedInput|/Game/TestSkillbox/Input/Action/IA_Move`
  (params (ActionValue :type "Vector2D Structure") (ElapsedSeconds :type "Float (double-precision)") (TriggeredSeconds :type "Float (double-precision)") (InputAction :type "InputAction Object Reference" :default "/Game/TestSkillbox/Input/Action/IA_Move.IA_Move"))
  (bind (_returnvalue_roll _returnvalue_pitch _returnvalue_yaw) (`KismetMathLibrary.BreakRotator` (`self.GetControlRotation`)))
  ;[0 0 0] Движение игрока
  (:`Triggered`
    (bind _testskillbox_p (`/Game/TestSkillbox/Blueprint/DataAsset/PDA_GameplayClasses.TestSkillbox_P` (`self.GameplayClasses`))
      (:`then`
        (`Pawn.AddMovementInput` _testskillbox_p (`KismetMathLibrary.GreaterGreater_VectorRotator` (`KismetMathLibrary.Conv_Vector2DToVector` ActionValue) (`KismetMathLibrary.MakeRotator` 0.0 0.0 _returnvalue_yaw)) 1.0 false))
      (:`else`))))

(event `EnhancedInput|/Game/TestSkillbox/Input/Action/IA_Look`
  (params (ActionValue :type "Vector2D Structure") (ElapsedSeconds :type "Float (double-precision)") (TriggeredSeconds :type "Float (double-precision)") (InputAction :type "InputAction Object Reference" :default "/Game/TestSkillbox/Input/Action/IA_Look.IA_Look"))
  ;[0 0 0] Движение камерой
  (:`Triggered`
    (`self.AddYawInput` ActionValue_X)
    (`self.AddPitchInput` ActionValue_Y)))

(event `EnhancedInput|/Game/TestSkillbox/Input/Action/IA_Jump`
  (params (ActionValue :type Boolean) (ElapsedSeconds :type "Float (double-precision)") (TriggeredSeconds :type "Float (double-precision)") (InputAction :type "InputAction Object Reference" :default "/Game/TestSkillbox/Input/Action/IA_Jump.IA_Jump"))
  ;[0 0 0] Прыжок
  (:`Started`
    (bind _testskillbox_p (`/Game/TestSkillbox/Blueprint/DataAsset/PDA_GameplayClasses.TestSkillbox_P` (`self.GameplayClasses`))
      (:`then`
        (if (not (`/Game/TestSkillbox/Core/BP_TestSkillbox_P.Mode Shoot` _testskillbox_p))
          (`/Game/TestSkillbox/Blueprint/Character/BP_BaseCharacter.ActiveAbility` _testskillbox_p true "/Game/TestSkillbox/Blueprint/AbilitySystem/GA_Jump.GA_Jump_C")))
      (:`else`))))

(event `EnhancedInput|/Game/TestSkillbox/Input/Action/IA_Pause`
  (params (ActionValue :type Boolean) (ElapsedSeconds :type "Float (double-precision)") (TriggeredSeconds :type "Float (double-precision)") (InputAction :type "InputAction Object Reference" :default "/Game/TestSkillbox/Input/Action/IA_Pause.IA_Pause"))
  ;[0 0 0] Пауза
  (:`Completed`
    (`/Game/TestSkillbox/Core/BP_TestSkillBox_GM.SetGamePause` (`/Game/TestSkillbox/Blueprint/DataAsset/PDA_GameplayClasses.TestSkillbox_GM` (`self.GameplayClasses`)) true)))

(event `EnhancedInput|/Game/TestSkillbox/Input/Action/IA_Sprint`
  (params (ActionValue :type Boolean) (ElapsedSeconds :type "Float (double-precision)") (TriggeredSeconds :type "Float (double-precision)") (InputAction :type "InputAction Object Reference" :default "/Game/TestSkillbox/Input/Action/IA_Sprint.IA_Sprint"))
  (bind _gameplayclasses (`self.GameplayClasses`))
  ;[0 0 0] Спринт
  (:`Started`
    (bind _testskillbox_p (`/Game/TestSkillbox/Blueprint/DataAsset/PDA_GameplayClasses.TestSkillbox_P` _gameplayclasses)
      (:`then`
        (`/Game/TestSkillbox/Blueprint/Character/BP_BaseCharacter.ActiveAbility` _testskillbox_p true "/Game/TestSkillbox/Blueprint/AbilitySystem/GA_Sprint.GA_Sprint_C"))
      (:`else`)))
  (:`Completed`
    (bind _testskillbox_p_2 (`/Game/TestSkillbox/Blueprint/DataAsset/PDA_GameplayClasses.TestSkillbox_P` _gameplayclasses)
      (:`then`
        (`/Game/TestSkillbox/Blueprint/Character/BP_BaseCharacter.ActiveAbility` _testskillbox_p_2 false "/Game/TestSkillbox/Blueprint/AbilitySystem/GA_Sprint.GA_Sprint_C"))
      (:`else`))))

(event `EnhancedInput|/Game/TestSkillbox/Input/Action/IA_Management`
  (params (ActionValue :type Boolean) (ElapsedSeconds :type "Float (double-precision)") (TriggeredSeconds :type "Float (double-precision)") (InputAction :type "InputAction Object Reference" :default "/Game/TestSkillbox/Input/Action/IA_Management.IA_Management"))
  (bind _gameplayclasses (`self.GameplayClasses`))
  ;[0 0 0] Показ подсказки управления
  (:`Started`
    (bind _testskillbox_hud (`/Game/TestSkillbox/Blueprint/DataAsset/PDA_GameplayClasses.TestSkillbox_HUD` _gameplayclasses)
      (:`then`
        (`/Game/TestSkillbox/Core/BP_TestSkillbox_HUD.ShowManagement` _testskillbox_hud true))
      (:`else`)))
  (:`Completed`
    (bind _testskillbox_hud_2 (`/Game/TestSkillbox/Blueprint/DataAsset/PDA_GameplayClasses.TestSkillbox_HUD` _gameplayclasses)
      (:`then`
        (`/Game/TestSkillbox/Core/BP_TestSkillbox_HUD.ShowManagement` _testskillbox_hud_2 false))
      (:`else`))))

(event `EnhancedInput|/Game/TestSkillbox/Input/Action/IA_Fix`
  (params (ActionValue :type Boolean) (ElapsedSeconds :type "Float (double-precision)") (TriggeredSeconds :type "Float (double-precision)") (InputAction :type "InputAction Object Reference" :default "/Game/TestSkillbox/Input/Action/IA_Fix.IA_Fix"))
  (bind _gameplayclasses (`self.GameplayClasses`))
  ;[0 0 0] Взаимодействие
  (:`Started`
    (bind _testskillbox_p (`/Game/TestSkillbox/Blueprint/DataAsset/PDA_GameplayClasses.TestSkillbox_P` _gameplayclasses)
      (:`then`
        (`/Game/TestSkillbox/Blueprint/Character/BP_BaseCharacter.ActiveAbility` _testskillbox_p true "/Game/TestSkillbox/Blueprint/AbilitySystem/GA_Fix.GA_Fix_C"))
      (:`else`)))
  (:`Completed`
    (bind _testskillbox_p_2 (`/Game/TestSkillbox/Blueprint/DataAsset/PDA_GameplayClasses.TestSkillbox_P` _gameplayclasses)
      (:`then`
        (`/Game/TestSkillbox/Blueprint/Character/BP_BaseCharacter.ActiveAbility` _testskillbox_p_2 false "/Game/TestSkillbox/Blueprint/AbilitySystem/GA_Fix.GA_Fix_C"))
      (:`else`))))

(event `EnhancedInput|/Game/TestSkillbox/Input/Action/IA_Crouch`
  (params (ActionValue :type Boolean) (ElapsedSeconds :type "Float (double-precision)") (TriggeredSeconds :type "Float (double-precision)") (InputAction :type "InputAction Object Reference" :default "/Game/TestSkillbox/Input/Action/IA_Crouch.IA_Crouch"))
  (bind _returnvalue (`BlueprintGameplayTagLibrary.HasTag` (`GameplayTagAssetInterface.GetOwnedGameplayTags` (`/Game/TestSkillbox/Blueprint/Character/BP_BaseCharacter.AbilitySystem` (`/Game/TestSkillbox/Blueprint/DataAsset/PDA_GameplayClasses.TestSkillbox_P` (`self.GameplayClasses`)))) (struct :`TagName` "Status.Character.Crouch")))
  ;[0 0 0] Присест
  (:`Started`
    (bind _testskillbox_p (`/Game/TestSkillbox/Blueprint/DataAsset/PDA_GameplayClasses.TestSkillbox_P` (`self.GameplayClasses`))
      (:`then`
        (`/Game/TestSkillbox/Blueprint/Character/BP_BaseCharacter.ActiveAbility` _testskillbox_p (not _returnvalue) "/Game/TestSkillbox/Blueprint/AbilitySystem/GA_Crouch.GA_Crouch_C")
        (`SceneComponent.K2_SetRelativeLocation` (`/Game/TestSkillbox/Core/BP_TestSkillbox_P.Scene` _testskillbox_p) (`KismetMathLibrary.MakeVector` 0.0 0.0 (`KismetMathLibrary.SelectFloat` 48.0 0.0 _returnvalue)) false false))
      (:`else`))))

(event `EnhancedInput|/Game/TestSkillbox/Input/Action/IA_Reload`
  (params (ActionValue :type Boolean) (ElapsedSeconds :type "Float (double-precision)") (TriggeredSeconds :type "Float (double-precision)") (InputAction :type "InputAction Object Reference" :default "/Game/TestSkillbox/Input/Action/IA_Reload.IA_Reload"))
  ;[0 0 0] Перезарядка
  (:`Started`
    (bind _testskillbox_p (`/Game/TestSkillbox/Blueprint/DataAsset/PDA_GameplayClasses.TestSkillbox_P` (`self.GameplayClasses`))
      (:`then`
        (`/Game/TestSkillbox/Blueprint/Character/BP_BaseCharacter.ActiveAbility` _testskillbox_p true "/Game/TestSkillbox/Blueprint/AbilitySystem/GA_Reload.GA_Reload_C"))
      (:`else`))))

(event `EnhancedInput|/Game/TestSkillbox/Input/Action/IA_Shoot`
  (params (ActionValue :type Boolean) (ElapsedSeconds :type "Float (double-precision)") (TriggeredSeconds :type "Float (double-precision)") (InputAction :type "InputAction Object Reference" :default "/Game/TestSkillbox/Input/Action/IA_Shoot.IA_Shoot"))
  ;[0 0 0] Стрельба
  (:`Started`
    (`|ExecutionSequence`
      (:`then_0`
        (goto _label :!via `Open`))
      (:`then_1`
        (`/Engine/EditorBlueprintResources/StandardMacros.Gate` true :!label _label
          (:`Exit`
            (bind _testskillbox_p (`/Game/TestSkillbox/Blueprint/DataAsset/PDA_GameplayClasses.TestSkillbox_P` (`self.GameplayClasses`))
              (:`then`
                (if (not (`/Game/TestSkillbox/Blueprint/Character/BP_BaseCharacter.bDeath` _testskillbox_p))
                  (`/Game/TestSkillbox/Blueprint/Character/BP_BaseCharacter.ActiveAbility` _testskillbox_p true "/Game/TestSkillbox/Blueprint/AbilitySystem/GA_PlayerShoot.GA_PlayerShoot_C")
                  (`KismetSystemLibrary.Delay` 0.1)
                  (`|ExecutionSequence`
                    (:`then_0`
                      (goto _label)))))
              (:`else`)))))))
  (:`Completed`
    (goto _label :!via `Close`)))

(event `EnhancedInput|/Game/TestSkillbox/Input/Action/IA_Aim`
  (params (ActionValue :type Boolean) (ElapsedSeconds :type "Float (double-precision)") (TriggeredSeconds :type "Float (double-precision)") (InputAction :type "InputAction Object Reference" :default "/Game/TestSkillbox/Input/Action/IA_Aim.IA_Aim"))
  (bind _gameplayclasses (`self.GameplayClasses`))
  (bind _testskillbox_p (`/Game/TestSkillbox/Blueprint/DataAsset/PDA_GameplayClasses.TestSkillbox_P` (`self.GameplayClasses`)))
  (bind _tagcontainer (`GameplayTagAssetInterface.GetOwnedGameplayTags` (`/Game/TestSkillbox/Blueprint/Character/BP_BaseCharacter.AbilitySystem` (`/Game/TestSkillbox/Blueprint/DataAsset/PDA_GameplayClasses.TestSkillbox_P` _gameplayclasses))))
  ;[0 0 0] Режим стрельбы
  (:`Started`
    (bind _testskillbox_p_2 (`/Game/TestSkillbox/Blueprint/DataAsset/PDA_GameplayClasses.TestSkillbox_P` _gameplayclasses)
      (:`then`
        (bind _mode_shoot (`/Game/TestSkillbox/Core/BP_TestSkillbox_P.Mode Shoot` _testskillbox_p_2))
        (if (not _mode_shoot)
          (`|ExecutionSequence`
            (:`then_0`
              (goto _label_2 :!via `Open`))
            (:`then_1`
              (`KismetSystemLibrary.Delay` 0.15)
              (`/Engine/EditorBlueprintResources/StandardMacros.Gate` true :!label _label_2
                (:`Exit`
                  (bind _testskillbox_p_3 (`/Game/TestSkillbox/Blueprint/DataAsset/PDA_GameplayClasses.TestSkillbox_P` (`self.GameplayClasses`))
                    (:`then`
                      (bind _tagcontainer_2 (`GameplayTagAssetInterface.GetOwnedGameplayTags` (`/Game/TestSkillbox/Blueprint/Character/BP_BaseCharacter.AbilitySystem` _testskillbox_p_2)))
                      (if (and (not (`BlueprintGameplayTagLibrary.HasTag` _tagcontainer_2 (struct :`TagName` "Status.Character.Crouch"))) (not (`/Game/TestSkillbox/Blueprint/Character/BP_BaseCharacter.bDeath` _testskillbox_p_3)))
                        (if (not (`BlueprintGameplayTagLibrary.HasTag` _tagcontainer_2 (struct :`TagName` "Status.Character.ModeShoot")))
                          (`/Game/TestSkillbox/Core/BP_TestSkillbox_P.ModeShoot` _testskillbox_p_3 true)
                          (`|ExecutionSequence`
                            (:`then_0`
                              (goto _label_3 :!via `Open`))
                            (:`then_1`
                              (`KismetSystemLibrary.Delay` 1.2)
                              (`/Engine/EditorBlueprintResources/StandardMacros.Gate` true :!label _label_3
                                (:`Exit`
                                  _)))))
                        (`/Game/TestSkillbox/Blueprint/Character/BP_BaseCharacter.ActiveAbility` (`/Game/TestSkillbox/Blueprint/DataAsset/PDA_GameplayClasses.TestSkillbox_P` (`self.GameplayClasses`)) true "/Game/TestSkillbox/Blueprint/AbilitySystem/GA_Aim.GA_Aim_C")))
                    (:`else`))))))))
      (:`else`)))
  (:`Completed`
    (`/Game/TestSkillbox/Blueprint/DataAsset/PDA_GameplayClasses.TestSkillbox_P` _gameplayclasses
      (:`then`
        (if (not _mode_shoot)
          (`|ExecutionSequence`
            (:`then_0`
              (goto _label_2 :!via `Close`))
            (:`then_1`
              (goto _label_3 :!via `Close`))
            (:`then_2`
              (bind _testskillbox_p_4 (`/Game/TestSkillbox/Blueprint/DataAsset/PDA_GameplayClasses.TestSkillbox_P` (`self.GameplayClasses`))
                (:`then`
                  (if (and (not (`/Game/TestSkillbox/Blueprint/Character/BP_BaseCharacter.bDeath` _testskillbox_p_4)) (not (`BlueprintGameplayTagLibrary.HasTag` _tagcontainer (struct :`TagName` "Status.Character.Crouch"))))
                    (if (`BlueprintGameplayTagLibrary.HasTag` _tagcontainer (struct :`TagName` "Status.Character.ModeShoot"))
                      (if (`BlueprintGameplayTagLibrary.HasTag` (`GameplayTagAssetInterface.GetOwnedGameplayTags` (`/Game/TestSkillbox/Blueprint/Character/BP_BaseCharacter.AbilitySystem` (`/Game/TestSkillbox/Blueprint/DataAsset/PDA_GameplayClasses.TestSkillbox_P` (`self.GameplayClasses`)))) (struct :`TagName` "Status.Character.Aim"))
                        (`/Game/TestSkillbox/Blueprint/Character/BP_BaseCharacter.ActiveAbility` _testskillbox_p false "/Game/TestSkillbox/Blueprint/AbilitySystem/GA_Aim.GA_Aim_C")
                        (else
                          (`/Game/TestSkillbox/Core/BP_TestSkillbox_P.ModeShoot` _testskillbox_p false)))
                      (else
                        (`/Game/TestSkillbox/Core/BP_TestSkillbox_P.ModeShoot` (`/Game/TestSkillbox/Blueprint/DataAsset/PDA_GameplayClasses.TestSkillbox_P` (`self.GameplayClasses`)) true)))))
                (:`else`))))))
      (:`else`))))

(fn `IsAimActive`
  (returns (ReturnValue :type Boolean))
  ;[0 0 0] Получение информации о активности прицеливания
  (return (`|GetInputActionValue`)))

(fn `UserConstructionScript`)