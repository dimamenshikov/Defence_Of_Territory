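; Game instance for the TestSkillbox game that persists the player's record and provides access to game settings.
; On Init it registers itself in GameplayClasses and loads the saved record from a save slot.
; SaveRecord creates a BP_SaveRecord object when none is valid, then writes the new value to that slot.
; GetGameSetting returns the engine's GameUserSettings alongside the GameSetting variable.
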(event `self.ReceiveInit`
  ;[0 0 0] Запись себя в геймплейный класс, загрузка рекорда
  (set `/Game/TestSkillbox/Blueprint/DataAsset/PDA_GameplayClasses.TestSkillbox_GI` self (`self.GameplayClasses`))
  (`self.LoadGame`))

(fn `GetGameSetting`
  (returns (GameUserSetting :type "GameUserSettings Object Reference") (GameSetting :type "/Game/TestSkillbox/Blueprint/Structure/S_GameSetting Structure"))
  ;[0 0 0] Получение настроек игры
  (bind _returnvalue (`GameUserSettings.GetGameUserSettings`))
  (return _returnvalue (`self.GameSetting`)))

(fn `LoadGame`
  ;[0 0 0] Загрузка рекорда
  (bind _returnvalue (`GameplayStatics.LoadGameFromSlot` (`self.Slot Name`)))
  (bind _asbp_save_record (cast `/Game/TestSkillbox/Core/BP_SaveRecord` _returnvalue))
  (bind _output_get (set `self.SaveRecords` _asbp_save_record))
  (set `self.Record` (`/Game/TestSkillbox/Core/BP_SaveRecord.Record` _output_get)))

(fn `SaveRecord`
  (params (Record :type "Float (double-precision)"))
  (bind _saverecords (`self.SaveRecords`))
  ;[0 0 0] Сохранение рекорда
  (`self.SaveRecords`
    (:`then`
      _)
    (:`else`
      (bind _returnvalue (`GameplayStatics.CreateSaveGameObject` "/Game/TestSkillbox/Core/BP_SaveRecord.BP_SaveRecord_C"))
      (set `self.SaveRecords` _returnvalue)))
  (set `/Game/TestSkillbox/Core/BP_SaveRecord.Record` Record _saverecords)
  (`GameplayStatics.SaveGameToSlot` _saverecords (`self.Slot Name`)))