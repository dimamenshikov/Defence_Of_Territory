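; BP_Life is a health component that tracks damage taken by its owning actor.
; On BeginPlay it binds Damage to the owner's OnTakeAnyDamage, subtracting each hit from Health and clamping between zero and MaxHealth.
; It broadcasts the UpdateHealth dispatcher with the new value, normalized ratio and owner.
; For positive damage it also calls DamageMessage on the owner with the damage and remaining health.
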(event `self.ReceiveBeginPlay`
  ;[0 0 0] Подписка на получение урона владельцем
  (add `Actor.OnTakeAnyDamage` (`self.GetOwner`) (`|CreateDelegate` :!event `Damage`)))

(fn `Damage`
  (params (DamagedActor :type "Actor Object Reference") (Damage :type "Float (single-precision)") (DamageType :type "DamageType Object Reference") (InstigatedBy :type "Controller Object Reference") (DamageCauser :type "Actor Object Reference"))
  (bind _returnvalue (`self.GetOwner`))
  (bind _maxhealth (`self.MaxHealth`))
  ;[0 0 0] Изменение здоровья владельца
  (bind _output_get (set `self.Health` (`KismetMathLibrary.FClamp` (- (`self.Health`) Damage) 0.0 _maxhealth)))
  (`self.OnUpdateHealth` _output_get (/ _output_get _maxhealth) _returnvalue)
  (if (> Damage 0.0)
    (message `/Game/TestSkillbox/Blueprint/Interface/BPI_Damage.Damage` _returnvalue Damage (`self.Health`))))