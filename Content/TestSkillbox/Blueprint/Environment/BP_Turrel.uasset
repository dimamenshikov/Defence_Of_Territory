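; Turret Blueprint that automatically targets and shoots BP_Enemy actors, one at a time.
; It acquires targets by a sphere trace on BeginPlay or target loss, and by Sphere overlap when the current one is invalid or dead.
; Shoot turns the Turrel component's yaw toward the target each tick through a DelayUntilNextTick loop.
; Once aligned, it waits briefly, then applies damage directly with explosion and sound at the enemy, repeating until death.
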(event `self.ReceiveBeginPlay`
  ;[0 0 0] Нахождение врага по близости
  (`self.FindEnemy`))

(event `FindEnemy`
  (bind _returnvalue (`self.K2_GetActorLocation`))
  ;[0 0 0] Нахождение врага по близости
  (set `self.BP_Enemy` null)
  (bind _outhit (`KismetSystemLibrary.SphereTraceSingle` _returnvalue _returnvalue 1000.0 "TraceTypeQuery1"))
  (bind _asbp_enemy (cast `/Game/TestSkillbox/Blueprint/AI/Enemy/BP_Enemy` (`.HitActor` (`GameplayStatics.BreakHitResult` _outhit))))
  (bind _output_get (set `self.BP_Enemy` _asbp_enemy))
  (if (not (== (`/Game/TestSkillbox/Blueprint/Components/BP_Life.Health` (`/Game/TestSkillbox/Blueprint/Character/BP_BaseCharacter.BP_Life` _output_get)) 0.0))
    (`self.Shoot`)))

(event `self.Sphere.OnComponentBeginOverlap`
  (params (OverlappedComponent :type "PrimitiveComponent Object Reference") (OtherActor :type "Actor Object Reference") (OtherComp :type "PrimitiveComponent Object Reference") (OtherBodyIndex :type Integer) (bFromSweep :type Boolean) (SweepResult :type "HitResult Structure (by ref)"))
  ;[0 0 0] Сохранение ссылки на врага
  (bind _bp_enemy (`self.BP_Enemy`)
    (:`then`
      (if (== (`/Game/TestSkillbox/Blueprint/Components/BP_Life.Health` (`/Game/TestSkillbox/Blueprint/Character/BP_BaseCharacter.BP_Life` _bp_enemy)) 0.0)
        (bind _asbp_enemy (cast `/Game/TestSkillbox/Blueprint/AI/Enemy/BP_Enemy` OtherActor :!label _label))
        (set `self.BP_Enemy` _asbp_enemy)
        (`self.Shoot`)))
    (:`else`
      (goto _label))))

(event `Shoot`
  (bind _returnvalue (`self.K2_GetActorLocation` (`self.BP_Enemy`)))
  (bind (_relativerotation_roll _relativerotation_pitch _relativerotation_yaw) (`KismetMathLibrary.BreakRotator` (`SceneComponent.RelativeRotation` (`self.Turrel`))))
  (bind (_returnvalue_roll _returnvalue_pitch _returnvalue_yaw) (`KismetMathLibrary.BreakRotator` (`KismetMathLibrary.FindLookAtRotation` (`SceneComponent.K2_GetComponentLocation` (`self.Turrel`)) (`self.K2_GetActorLocation` (`self.BP_Enemy`)))))
  (bind _returnvalue_2 (- _returnvalue_yaw 90.0))
  ;[0 0 0] Поворот и стрельба по врагу
  (`self.BP_Enemy` :!label _label_2
    (:`then`
      (`SceneComponent.K2_SetRelativeRotation` (`self.Turrel`) (`KismetMathLibrary.MakeRotator` 0.0 0.0 (`KismetMathLibrary.FInterpTo_Constant` _relativerotation_yaw _returnvalue_2 (`GameplayStatics.GetWorldDeltaSeconds`) 200.0)) false false)
      (if (< (`KismetMathLibrary.Abs` (- _relativerotation_yaw _returnvalue_2)) 0.01)
        (`KismetSystemLibrary.Delay` 0.2)
        (`GameplayStatics.SpawnEmitterAtLocation` "/Game/TestSkillbox/Assets/Effect/Explosion/P_Explosion.P_Explosion" _returnvalue (struct) (0.5 0.5 0.5))
        (`GameplayStatics.PlaySoundAtLocation` "/Game/TestSkillbox/Assets/Audio/A_Shoot.A_Shoot" _returnvalue (struct) 1.0 1.0 0.0 null null null null)
        (`GameplayStatics.ApplyDamage` (`self.BP_Enemy`) (`self.Base Damage`))
        (`self.BP_Enemy`
          (:`then`
            (if (== (`/Game/TestSkillbox/Blueprint/Components/BP_Life.Health` (`/Game/TestSkillbox/Blueprint/Character/BP_BaseCharacter.BP_Life` (`self.BP_Enemy`))) 0.0)
              _
              (else
                (`KismetSystemLibrary.DelayUntilNextTick` :!label _label_3)
                (goto _label_2))))
          (:`else`
            _))
        (`self.FindEnemy`)
        (else
          (goto _label_3))))
    (:`else`
      (`self.FindEnemy`))))

(fn `UserConstructionScript`)