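; Bonus pickup actor that optionally spins around its vertical axis and is collected when the player pawn overlaps it.
; BeginPlay caches the game difficulty from the game instance, and Tick applies the frame-rate-independent yaw rotation.
; The first player overlap plays a sound scaled by the saved volume settings, then calls BonusActivate with the player, which here only destroys the actor.
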(event `self.ReceiveBeginPlay`
  ;[0 0 0] Получение сложности игры
  (set `self.GameDifficulty` (`/Game/TestSkillbox/Core/BP_TestSkillbox_GI.GameDifficulty` (`/Game/TestSkillbox/Blueprint/DataAsset/PDA_GameplayClasses.TestSkillbox_GI` (`self.GameplayClasses`)))))

(event `self.ReceiveTick`
  (params (DeltaSeconds :type "Float (single-precision)"))
  ;[0 0 0] Вращение бонуса
  (if (`self.Rotate`)
    (`self.K2_AddActorWorldRotation` (`KismetMathLibrary.MakeRotator` 0.0 0.0 (* DeltaSeconds 300.0)))))

(event `self.Bonus.OnComponentBeginOverlap`
  (params (OverlappedComponent :type "PrimitiveComponent Object Reference") (OtherActor :type "Actor Object Reference") (OtherComp :type "PrimitiveComponent Object Reference") (OtherBodyIndex :type Integer) (bFromSweep :type Boolean) (SweepResult :type "HitResult Structure (by ref)"))
  (bind (_gamesetting_sound _gamesetting_music _gamesetting_audio) (break `/Game/TestSkillbox/Blueprint/Structure/S_GameSetting` (`/Game/TestSkillbox/Core/BP_TestSkillbox_GI.GameSetting` (`/Game/TestSkillbox/Blueprint/DataAsset/PDA_GameplayClasses.TestSkillbox_GI` (`self.GameplayClasses`)))))
  ;[0 0 0] Подбор бонуса игроком, активация бонуса
  (bind _asbp_test_skillbox_p (cast `/Game/TestSkillbox/Core/BP_TestSkillbox_P` OtherActor))
  (`/Engine/EditorBlueprintResources/StandardMacros.DoOnce` false
    (:`Completed`
      (`GameplayStatics.PlaySoundAtLocation` (`self.Sound`) (`self.K2_GetActorLocation`) (struct) (* _gamesetting_sound _gamesetting_audio) 1.0 0.0 null null null null)
      (`self.Bonus Activate` _asbp_test_skillbox_p))))

(fn `Bonus Activate`
  (params (Player :type "/Game/TestSkillbox/Core/BP_TestSkillbox_P Object Reference"))
  ;[0 0 0] Активация бонуса
  (`self.K2_DestroyActor`))

(fn `UserConstructionScript`)