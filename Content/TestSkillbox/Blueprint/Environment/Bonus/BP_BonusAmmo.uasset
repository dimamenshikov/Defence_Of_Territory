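; BP_BonusAmmo is an ammo pickup that adds reserve rounds to the collecting player's active weapon.
; Its Bonus Activate override scales the configured amount by game difficulty, granting more on Easy and less on Hard.
; It then fires the weapon's ammo update call with magazine and reserve counts before running the parent bonus logic.
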(fn `Bonus Activate`
  (params (Player :type "/Game/TestSkillbox/Core/BP_TestSkillbox_P Object Reference"))
  (bind _activeweapon (`/Game/TestSkillbox/Blueprint/Character/BP_BaseCharacter.ActiveWeapon` Player))
  ;[0 0 0] Увеличение количества патронов
  (bind _output_get (set `/Game/TestSkillbox/Blueprint/Environment/BP_Weapon.PatronsInBag` (+ (`/Game/TestSkillbox/Blueprint/Environment/BP_Weapon.PatronsInBag` _activeweapon) (* (`self.QuantityAddPatrons`) (select `/Game/TestSkillbox/Blueprint/Enum/E_GameDifficulty` (`self.GameDifficulty`) :`NewEnumerator0` 1.25 :`NewEnumerator1` 1.0 :`NewEnumerator2` 0.75))) _activeweapon))
  (`/Game/TestSkillbox/Blueprint/Environment/BP_Weapon.UpdateAmmo` _activeweapon (`/Game/TestSkillbox/Blueprint/Environment/BP_Weapon.PatronsCurrentInShop` _activeweapon) _output_get)
  (`parent.Bonus Activate` Player))

(fn `UserConstructionScript`
  (`parent.UserConstructionScript`))