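; Bonus aura that, once activated, attaches to the player, healing them and damaging enemies within its area.
; BonusActivate destroys any attached aura of the same class, then scales up, turns green and starts healing.
; Overlap events maintain the enemy array, and each enemy entry starts the damage loop.
; Both effects use ApplyDamage in self-calling 0.2-second Delay loops, with healing passing the Healing value as damage.
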(event `PlayerHealing`
  ;[0 0 0] Лечение игрока
  (bind _playerowner (`self.PlayerOwner`)
    (:`then`
      (`GameplayStatics.ApplyDamage` _playerowner (`self.Healing`))
      (`KismetSystemLibrary.Delay` 0.2)
      (`self.PlayerHealing`))
    (:`else`)))

(event `Damage`
  ;[0 0 0] Урон врагам
  (for _array_element (`self.Enemy`)
    (`GameplayStatics.ApplyDamage` _array_element (`self.Base Damage`)))
  (`KismetSystemLibrary.Delay` 0.2)
  (if (`KismetArrayLibrary.Array_IsNotEmpty` (`self.Enemy`))
    (`self.Damage`)))

(event `self.Bonus.OnComponentBeginOverlap`
  (params (OverlappedComponent :type "PrimitiveComponent Object Reference") (OtherActor :type "Actor Object Reference") (OtherComp :type "PrimitiveComponent Object Reference") (OtherBodyIndex :type Integer) (bFromSweep :type Boolean) (SweepResult :type "HitResult Structure (by ref)"))
  ;[0 0 0] Запись ссылок врагов в массив
  (bind _asbp_enemy (cast `/Game/TestSkillbox/Blueprint/AI/Enemy/BP_Enemy` OtherActor))
  (`KismetArrayLibrary.Array_Add` (`self.Enemy`) _asbp_enemy)
  (`self.Damage`))

(event `self.Bonus.OnComponentEndOverlap`
  (params (OverlappedComponent :type "PrimitiveComponent Object Reference") (OtherActor :type "Actor Object Reference") (OtherComp :type "PrimitiveComponent Object Reference") (OtherBodyIndex :type Integer))
  ;[0 0 0] Удаление врага из массива при выходе из ауры
  (set `self.Num` -1)
  (for _array_element (`self.Enemy`)
    (if (== _array_element OtherActor)
      (set `self.Num` 0)
      (break)))
  (if (!= (`self.Num`) -1)
    (`KismetArrayLibrary.Array_RemoveItem` (`self.Enemy`) (`|GetArrayItem` (`self.Enemy`) (`self.Num`)))))

(fn `Bonus Activate`
  (params (Player :type "/Game/TestSkillbox/Core/BP_TestSkillbox_P Object Reference"))
  (bind _bonus (`self.Bonus`))
  ;[0 0 0] Активация ауры
  (for _array_element (`self.GetAttachedActors` Player true false)
    (if (== (`GameplayStatics.GetObjectClass` _array_element) (`GameplayStatics.GetObjectClass` self))
      (`self.K2_DestroyActor` _array_element)))
  (bind _output_get (set `self.PlayerOwner` Player))
  (`self.K2_AttachToActor` _output_get "None" "KeepRelative" "KeepRelative" "KeepRelative")
  (`self.K2_SetActorRelativeTransform` (`KismetMathLibrary.MakeTransform` (0.0 0.0 0.0) (struct) (10.0 10.0 10.0)))
  (`SceneComponent.K2_SetRelativeTransform` _bonus (`KismetMathLibrary.MakeTransform` (0.0 0.0 0.0)) false false)
  (`PrimitiveComponent.SetMaterial` _bonus 0 "/Game/TestSkillbox/Assets/GlobalMaterial/MI_Green.MI_Green")
  (`self.PlayerHealing`))

(fn `UserConstructionScript`)