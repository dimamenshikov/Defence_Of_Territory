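; BP_Pill is a bonus pickup that restores the player's Health, which its graph comment frames as stress reduction.
; On activation it adds PatronsAdd scaled by a GameDifficulty multiplier, largest on Easy, and caps the result at MaxHealth.
; It then broadcasts OnUpdateHealth from the player's BPLife with the new value and fill ratio, and hands off to the parent BonusActivate.
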(fn `Bonus Activate`
  (params (Player :type "/Game/TestSkillbox/Core/BP_TestSkillbox_P Object Reference"))
  (bind _bp_life (`/Game/TestSkillbox/Blueprint/Character/BP_BaseCharacter.BP_Life` Player))
  (bind _maxhealth (`/Game/TestSkillbox/Blueprint/Components/BP_Life.MaxHealth` _bp_life))
  ;[0 0 0] Уменьшение стресса в зависимости от уровня сложности
  (bind _output_get (set `/Game/TestSkillbox/Blueprint/Components/BP_Life.Health` (`KismetMathLibrary.FMin` _maxhealth (+ (`/Game/TestSkillbox/Blueprint/Components/BP_Life.Health` _bp_life) (* (select `/Game/TestSkillbox/Blueprint/Enum/E_GameDifficulty` (`self.GameDifficulty`) :`NewEnumerator0` 1.25 :`NewEnumerator1` 1.0 :`NewEnumerator2` 0.75) (`self.PatronsAdd`)))) _bp_life))
  (`/Game/TestSkillbox/Blueprint/Components/BP_Life.OnUpdateHealth` _bp_life _output_get (/ _output_get _maxhealth) Player)
  (`parent.Bonus Activate` Player))

(fn `UserConstructionScript`
  (`parent.UserConstructionScript`))