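; BP_Arrow is an indicator arrow that shows the status of a referenced defence object.
; On BeginPlay, if that object is valid, it binds to its damage and destroyed events and starts a Timeline that moves the arrow vertically from its starting height.
; A dynamic material created in the construction script turns red on damage, with a timer to restore yellow.
; Destruction sets red and clears the timer, keeping the arrow red.
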(event `self.ReceiveBeginPlay`
  (bind (_returnvalue_x _returnvalue_y _returnvalue_z) (`KismetMathLibrary.BreakVector` (`self.K2_GetActorLocation`)))
  (bind (_returnvalue_x_2 _returnvalue_y_2) (`KismetMathLibrary.BreakVector` (`self.K2_GetActorLocation`)))
  ;[0 0 0] Подписка на изменение здоровья объекта, поднимание/опускание стелки
  (set `self.Start_Z` _returnvalue_z)
  (bind _defencesobject (`self.DefencesObject`)
    (:`then`
      (add `self.OnTakeAnyDamage` _defencesobject (`|CreateDelegate` :!event `AttackedObject`))
      (add `self.OnDestroyed` _defencesobject (`|CreateDelegate` :!event `SetRedColor`))
      (bind (_direction _z) (`Timeline|Timeline`)
        (:`Update`
          (`self.K2_SetActorLocation` (`KismetMathLibrary.MakeVector` _returnvalue_x_2 _returnvalue_y_2 (+ _z (`self.Start_Z`)))))))
    (:`else`)))

(event `AttackedObject` :!signature `self.OnTakeAnyDamage`
  (params (DamagedActor :type "Actor Object Reference") (Damage :type "Float (single-precision)") (DamageType :type "DamageType Object Reference") (InstigatedBy :type "Controller Object Reference") (DamageCauser :type "Actor Object Reference"))
  ;[0 0 0] Установка красного цвета стрелки при атаки объекта, сброс цвета
  (if (> Damage 0.0)
    (`MaterialInstanceDynamic.SetVectorParameterValue` (`self.Material`) "Color" (struct :`R` 1.0 :`A` 1.0))
    (bind _returnvalue (`KismetSystemLibrary.K2_SetTimerDelegate` (`|CreateDelegate` :!event `ReturnColor`) 3.0))
    (set `self.Timer` _returnvalue)))

(event `ReturnColor`
  ;[0 0 0] Установка красного цвета стрелки при атаки объекта, сброс цвета
  (`MaterialInstanceDynamic.SetVectorParameterValue` (`self.Material`) "Color" (struct :`R` 1.0 :`G` 1.0 :`A` 1.0)))

(event `SetRedColor` :!signature `self.OnDestroyed`
  (params (DestroyedActor :type "Actor Object Reference"))
  ;[0 0 0] Установка красного цвета при уничтожении объекта
  (`MaterialInstanceDynamic.SetVectorParameterValue` (`self.Material`) "Color" (struct :`R` 1.0 :`A` 1.0))
  (`KismetSystemLibrary.K2_ClearAndInvalidateTimerHandle` (`self.Timer`)))

(fn `UserConstructionScript`
  ;[0 0 0] Создание динамического материала
  (bind _returnvalue (`PrimitiveComponent.CreateDynamicMaterialInstance` (`self.Arrow`) 0 null "None"))
  (set `self.Material` _returnvalue))