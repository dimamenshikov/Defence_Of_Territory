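; BP_Box is an environment actor that builds a wall of boxes from its origin toward EndLocation.
; The construction script fills one instanced static mesh component with a grid of scaled boxes.
; EndLocation's horizontal length sets the column count and its height the row count, with at least one row.
; Columns follow the horizontal direction with slight gaps, and each box is yawed along that line.
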(fn `UserConstructionScript`
  (locals (Box :type "InstancedStaticMeshComponent Object Reference"))
  (bind _returnvalue (`self.K2_GetActorLocation`))
  (bind (_endlocation_x _endlocation_y) (`KismetMathLibrary.BreakVector` (`self.EndLocation`)))
  (bind (_endlocation_x_2 _endlocation_y_2 _endlocation_z) (`KismetMathLibrary.BreakVector` (`self.EndLocation`)))
  (bind (_returnvalue_roll _returnvalue_pitch _returnvalue_yaw) (`KismetMathLibrary.BreakRotator` (`KismetMathLibrary.FindLookAtRotation` _returnvalue (+ (`KismetMathLibrary.MakeVector` _endlocation_x _endlocation_y) _returnvalue))))
  (bind _returnvalue_2 (`KismetMathLibrary.FFloor` (/ (`KismetMathLibrary.VSize` (`KismetMathLibrary.MakeVector` _endlocation_x_2 _endlocation_y_2)) 150.0)))
  ;[0 0 0] Создание стены из ящиков по конечной точки
  (bind _returnvalue_3 (`AddComponent|NODE_AddInstancedStaticMeshComponent-0`))
  (set `local.Box` _returnvalue_3)
  (if (> _returnvalue_2 0)
    (for _index (range (`KismetMathLibrary.Max` (`KismetMathLibrary.FFloor` (/ _endlocation_z 150.0)) 1))
      (for _index_2 (range _returnvalue_2)
        (bind (_returnvalue_x _returnvalue_y) (`KismetMathLibrary.BreakVector` (* (`KismetMathLibrary.Normal` (`KismetMathLibrary.MakeVector` _endlocation_x _endlocation_y)) (+ (* _index_2 155) 75))))
        (`InstancedStaticMeshComponent.AddInstance` (`local.Box`) (`KismetMathLibrary.MakeTransform` (`KismetMathLibrary.MakeVector` _returnvalue_x _returnvalue_y (`KismetMathLibrary.Conv_IntToDouble` (+ (* _index 150) 75))) (`KismetMathLibrary.MakeRotator` 0.0 0.0 _returnvalue_yaw) (1.5 1.5 1.5)) false)))))