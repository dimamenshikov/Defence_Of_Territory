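; BP_Fence is an environment Blueprint that builds a straight fence toward an end point, EndLocation.
; Its construction script flattens EndLocation to the actor's Z and derives the segment count from the vector's length.
; It adds an Instanced Static Mesh component and places scaled instances at fixed steps along that direction, yawed to face the end point.
; The count divisor differs from the placement step.
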(fn `UserConstructionScript`
  (bind (_returnvalue_x _returnvalue_y _returnvalue_z) (`KismetMathLibrary.BreakVector` (`self.K2_GetActorLocation`)))
  (bind _returnvalue (`self.K2_GetActorLocation`))
  (bind (_endlocation_x _endlocation_y) (`KismetMathLibrary.BreakVector` (`self.EndLocation`)))
  (bind _endlocation (`self.EndLocation`))
  (bind (_returnvalue_roll _returnvalue_pitch _returnvalue_yaw) (`KismetMathLibrary.BreakRotator` (`KismetMathLibrary.FindLookAtRotation` _returnvalue (+ _returnvalue _endlocation))))
  ;[0 0 0] Создание забора по конечной точки
  (bind _output_get (set `self.EndLocation` (`KismetMathLibrary.MakeVector` _endlocation_x _endlocation_y _returnvalue_z)))
  (bind _returnvalue_2 (`AddComponent|NODE_AddInstancedStaticMeshComponent-1`))
  (set `self.Fence` _returnvalue_2)
  (bind _returnvalue_3 (`KismetMathLibrary.FFloor` (/ (`KismetMathLibrary.VSize` _output_get) 340.0)))
  (if (> _returnvalue_3 0)
    (for _index (range _returnvalue_3)
      (bind (_returnvalue_x_2 _returnvalue_y_2) (`KismetMathLibrary.BreakVector` (* (`KismetMathLibrary.Normal` _endlocation) (+ (* _index 225) 105))))
      (`InstancedStaticMeshComponent.AddInstance` (`self.Fence`) (`KismetMathLibrary.MakeTransform` (`KismetMathLibrary.MakeVector` _returnvalue_x_2 _returnvalue_y_2 75.0) (`KismetMathLibrary.MakeRotator` 0.0 0.0 _returnvalue_yaw) (1.5 1.5 1.5)) false))))