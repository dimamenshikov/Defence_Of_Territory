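; Projectile Blueprint that plays effects when it spawns and when it hits a target.
; BeginPlay spawns a particle emitter and sound, then scales Damage by the owning weapon's character BaseDamageCoefficient.
; Exterminate plays a separate impact emitter and sound, with both sounds' volume scaled by the game's Sound and Audio settings.
; Shoot is empty, and no movement, collision or damage application is scripted in these graphs.
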(event `Shoot`
  ;[0 0 0] Проигрывание эффектов при создании и попаданиив цель
)

(event `self.ReceiveBeginPlay`
  (bind _returnvalue (`self.K2_GetActorLocation`))
  (bind (_usergamesetting _gamesetting) (`/Game/TestSkillbox/Blueprint/BlueprintFunctions.GetGameSetting`))
  ;[0 0 0] Проигрывание эффектов при создании и попаданиив цель
  (`GameplayStatics.SpawnEmitterAtLocation` (`self.Emitter Template`) _returnvalue (struct) (0.5 0.5 0.5))
  (`GameplayStatics.PlaySoundAtLocation` (`self.Sound`) _returnvalue (struct) (* (break `/Game/TestSkillbox/Blueprint/Structure/S_GameSetting` _gamesetting) (`.Audio_9_7DE9B5BF488BD0CA4371A8A2225B1AD7` (break `/Game/TestSkillbox/Blueprint/Structure/S_GameSetting` _gamesetting))) 1.0 0.0 null null null null)
  (set `self.Damage` (* (`/Game/TestSkillbox/Blueprint/Character/BP_BaseCharacter.BaseDamageCoefficient` (`/Game/TestSkillbox/Blueprint/Environment/BP_Weapon.CharacterOwner` (`self.Weapon`))) (`self.Damage`))))

(event `Exterminate`
  (bind _returnvalue (`self.K2_GetActorLocation`))
  (bind (_usergamesetting _gamesetting) (`/Game/TestSkillbox/Blueprint/BlueprintFunctions.GetGameSetting`))
  ;[0 0 0] Проигрывание эффектов при создании и попаданиив цель
  (`GameplayStatics.SpawnEmitterAtLocation` (`self.EmitterExterminate`) _returnvalue (struct) (0.25 0.25 0.25))
  (`GameplayStatics.PlaySoundAtLocation` (`self.SoundExterminate`) _returnvalue (struct) (* (break `/Game/TestSkillbox/Blueprint/Structure/S_GameSetting` _gamesetting) (`.Audio_9_7DE9B5BF488BD0CA4371A8A2225B1AD7` (break `/Game/TestSkillbox/Blueprint/Structure/S_GameSetting` _gamesetting))) 1.0 0.0 null null null null))

(fn `UserConstructionScript`)