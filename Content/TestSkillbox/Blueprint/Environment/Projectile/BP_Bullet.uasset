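; BP_Bullet is a projectile actor that delivers damage at the end point of a shot and then removes itself.
; On Shoot it waits a tick, jumps to End without sweeping, and damages the first overlapping actor, crediting the weapon's owning character.
; Without a valid Weapon, the damage call has no target or causer wired.
; It then calls Exterminate and destroys itself a tick later.
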(event `self.Shoot`
  (bind _damage (`self.Damage`))
  ;[0 0 0] Урон по пересеченному актору, уничтожении пули
  (`KismetSystemLibrary.DelayUntilNextTick`)
  (`self.K2_SetActorLocation` (`self.End`))
  (bind _weapon (`self.Weapon`)
    (:`then`
      (`GameplayStatics.ApplyDamage` (`|GetArrayItem` (`self.GetOverlappingActors` "/Script/Engine.Actor")) _damage null (`/Game/TestSkillbox/Blueprint/Environment/BP_Weapon.CharacterOwner` _weapon)))
    (:`else`
      (`GameplayStatics.ApplyDamage` null _damage)))
  (`self.Exterminate`)
  (`KismetSystemLibrary.DelayUntilNextTick`)
  (`self.K2_DestroyActor`))

(fn `UserConstructionScript`
  (`parent.UserConstructionScript`))