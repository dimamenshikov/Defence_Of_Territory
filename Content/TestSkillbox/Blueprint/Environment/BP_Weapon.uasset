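; BP_Weapon is a weapon Blueprint that handles magazine and reserve ammo, firing and reloading.
; Shoot spends a round, plays the owner's fire montage, spawns and launches a projectile toward an End parameter, and returns whether rounds remain.
; Reload tops up the magazine from the reserve, or only reports whether that is possible when CheckOnly is set.
; Both broadcast ammo counts through UpdateAmmo when they change.
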(fn `Reload`
  (params (CheckOnly :type Boolean))
  (returns (ReturnValue :type Boolean))
  (locals (Temp :type Integer :default 0))
  (bind _returnvalue (and (!= (`self.PatronsInBag`) 0) (!= (`self.PatronsCurrentInShop`) (`self.PatronsInShop`))))
  ;[0 0 0] Перезарядка
  (if CheckOnly
    (return _returnvalue)
    (elif _returnvalue
      (bind _output_get (set `local.Temp` (`KismetMathLibrary.Min` (- (`self.PatronsInShop`) (`self.PatronsCurrentInShop`)) (`self.PatronsInBag`))))
      (bind _output_get_2 (set `self.PatronsCurrentInShop` (+ (`self.PatronsCurrentInShop`) _output_get)))
      (bind _output_get_3 (set `self.PatronsInBag` (- (`self.PatronsInBag`) _output_get)))
      (`self.UpdateAmmo` _output_get_2 _output_get_3)
      (return true)
      (else
        (return false)))))

(fn `Shoot`
  (params (End :type "Vector Structure"))
  (returns (ExistPatrons :type Boolean))
  (bind _characterowner (`self.CharacterOwner`))
  ;[0 0 0] Создание снаряда, проигрывание анимации
  (if (!= (`self.PatronsCurrentInShop`) 0)
    (`/Engine/EditorBlueprintResources/StandardMacros.DecrementInt` (`self.PatronsCurrentInShop`)
      (:`  `
        (`Character.PlayAnimMontage` _characterowner (`self.AnimFire`) 1.0 "None")
        (bind _returnvalue (`|SpawnActorFromClass` (`self.ClassProjectile`) (`KismetMathLibrary.MakeTransform` (`self.K2_GetActorLocation` (`/Game/TestSkillbox/Blueprint/Character/BP_BaseCharacter.ActiveWeapon` _characterowner))) "Undefined" "MultiplyWithRoot" null self End null))
        (`/Game/TestSkillbox/Blueprint/Environment/BP_Projecile.Shoot` _returnvalue)
        (`self.UpdateAmmo` (`self.PatronsCurrentInShop`) (`self.PatronsInBag`))
        (return (> (`self.PatronsCurrentInShop`) 0))))
    (else
      (return (> (`self.PatronsCurrentInShop`) 0)))))

(fn `UserConstructionScript`)