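; BP_DefenceBlock is a destructible defence block that can be repaired through interaction.
; On BeginPlay it scales BPLife health and max health by game difficulty, making blocks tougher on Easy.
; At zero health it spawns explosion and fire effects with sounds at the game-settings volume, then destroys itself.
; Interaction plays a hammering sound and heals by applying negative damage, throttled by a DoOnce that resets after a one-second delay.
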(event `self.ReceiveBeginPlay`
  (bind _bp_life (`self.BP_Life`))
  ;[0 0 0] Установка жизней в зависимости от сложности
  (bind _output_get (set `/Game/TestSkillbox/Blueprint/Components/BP_Life.Health` (* (select `/Game/TestSkillbox/Blueprint/Enum/E_GameDifficulty` (`/Game/TestSkillbox/Core/BP_TestSkillbox_GI.GameDifficulty` (`/Game/TestSkillbox/Blueprint/DataAsset/PDA_GameplayClasses.TestSkillbox_GI` (`self.GameplayClasses`))) :`NewEnumerator0` 1.25 :`NewEnumerator1` 1.0 :`NewEnumerator2` 0.75) (`/Game/TestSkillbox/Blueprint/Components/BP_Life.Health` (`self.BP_Life`))) _bp_life))
  (set `/Game/TestSkillbox/Blueprint/Components/BP_Life.MaxHealth` _output_get _bp_life))

(event `/Game/TestSkillbox/Blueprint/Interface/BPI_Damage.Damage`
  (params (Damage :type "Float (double-precision)") (Health :type "Float (double-precision)"))
  (bind _returnvalue (`self.K2_GetActorLocation`))
  (bind (_gamesetting_sound _gamesetting_music _gamesetting_audio) (break `/Game/TestSkillbox/Blueprint/Structure/S_GameSetting` (`/Game/TestSkillbox/Core/BP_TestSkillbox_GI.GameSetting` (`/Game/TestSkillbox/Blueprint/DataAsset/PDA_GameplayClasses.TestSkillbox_GI` (`self.GameplayClasses`)))))
  (bind _returnvalue_2 (* _gamesetting_sound _gamesetting_audio))
  ;[0 0 0] Уничтожение объекта
  (if (== Health 0.0)
    (`GameplayStatics.SpawnEmitterAtLocation` "/Game/TestSkillbox/Assets/Effect/Explosion/P_Explosion.P_Explosion" _returnvalue (struct) (5.0 5.0 5.0))
    (`GameplayStatics.SpawnEmitterAtLocation` "/Game/TestSkillbox/Assets/Effect/Fire/Fire_00.Fire_00" _returnvalue (struct) (10.0 10.0 10.0) false)
    (`GameplayStatics.PlaySoundAtLocation` "/Game/TestSkillbox/Assets/Audio/Explosion01.Explosion01" _returnvalue (struct) _returnvalue_2 1.0 0.0 null null null null)
    (`GameplayStatics.SpawnSoundAtLocation` "/Game/TestSkillbox/Assets/Audio/Fire01.Fire01" _returnvalue (struct) _returnvalue_2 1.0 0.0 null null false)
    (`self.K2_DestroyActor`)))

(event `/Game/TestSkillbox/Blueprint/Interface/BPI_Interaction.Interaction`
  (bind (_gamesetting_sound _gamesetting_music _gamesetting_audio) (break `/Game/TestSkillbox/Blueprint/Structure/S_GameSetting` (`/Game/TestSkillbox/Core/BP_TestSkillbox_GI.GameSetting` (`/Game/TestSkillbox/Blueprint/DataAsset/PDA_GameplayClasses.TestSkillbox_GI` (`self.GameplayClasses`)))))
  ;[0 0 0] Починка объекта
  (`/Engine/EditorBlueprintResources/StandardMacros.DoOnce` false :!label _label
    (:`Completed`
      (`GameplayStatics.PlaySoundAtLocation` "/Game/TestSkillbox/Assets/Audio/hammering-on-the-door.hammering-on-the-door" (`self.K2_GetActorLocation`) (struct) (* _gamesetting_sound _gamesetting_audio) 1.0 0.0 "/Game/TestSkillbox/Assets/Audio/BaseSoundAttenuation.BaseSoundAttenuation" null null null)
      (`GameplayStatics.ApplyDamage` self (* (`self.Healing`) -1.0))
      (`KismetSystemLibrary.Delay` 1.0)
      (goto _label :!via `Reset`))))

(fn `UserConstructionScript`)