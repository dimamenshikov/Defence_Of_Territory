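; Wave manager actor that spawns enemy waves and ends the game as a win after the last one.
; On BeginPlay it waits for the player, converts spawn points to world space and scales enemy counts by difficulty.
; A looping timer spawns random enemy classes at random points until the wave quota is met.
; Death callbacks track living enemies; clearing a wave schedules the next and shows the upgrade widget.
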(event `self.ReceiveBeginPlay`
  (bind (_returnvalue_location _returnvalue_rotation) (`KismetMathLibrary.BreakTransform` (`self.GetTransform`)))
  ;[0 0 0] Перевод точек создания врагов в глобальные координаты
  (`/Game/TestSkillbox/Blueprint/DataAsset/PDA_GameplayClasses.TestSkillbox_P` (`self.GameplayClasses`) :!label _label
    (:`then`
      (set `self.CoefficientDifficulty` (select `/Game/TestSkillbox/Blueprint/Enum/E_GameDifficulty` (`/Game/TestSkillbox/Core/BP_TestSkillbox_GI.GameDifficulty` (`/Game/TestSkillbox/Blueprint/DataAsset/PDA_GameplayClasses.TestSkillbox_GI` (`self.GameplayClasses`))) :`NewEnumerator0` 0.75 :`NewEnumerator1` 1.0 :`NewEnumerator2` 1.25))
      (bind _returnvalue (`|CreateWidget` "/Game/TestSkillbox/Widget/WBP_Upgrate.WBP_Upgrate_C" null (`/Game/TestSkillbox/Blueprint/DataAsset/PDA_GameplayClasses.TestSkillbox_P` (`self.GameplayClasses`))))
      (set `self.Upgrate` _returnvalue)
      (for _array_element (`self.PointSpawn`)
        (`|VariableSetRef` _array_element (`KismetMathLibrary.MakeTransform` (+ (.location _array_element) _returnvalue_location) (`KismetMathLibrary.ComposeRotators` (.rotation _array_element) _returnvalue_rotation))))
      (if (`KismetArrayLibrary.Array_IsNotEmpty` (`self.Wave`))
        (for _array_element_2 (`self.Wave`)
          (setmembers `/Game/TestSkillbox/Blueprint/Structure/S_WaveSetting` :`StructRef` _array_element_2 :`Enemy` (`KismetMathLibrary.Round` (* (`.Enemy_13_A8C892F74FA6352906842A84461EAF5F` (break `/Game/TestSkillbox/Blueprint/Structure/S_WaveSetting` _array_element_2)) (`self.CoefficientDifficulty`)))))
        (`self.SpawnWave`)))
    (:`else`
      (`KismetSystemLibrary.DelayUntilNextTick`)
      (goto _label))))

(event `SpawnWave`
  (bind (_output_enemy _output_intervalspawnenemy) (break `/Game/TestSkillbox/Blueprint/Structure/S_WaveSetting` (`|GetArrayItem` (`self.Wave`) (- (`self.CurrentWave`) 1))))
  ;[0 0 0] Создание противников
  (bind _result (`/Engine/EditorBlueprintResources/StandardMacros.IncrementInt` (`self.CurrentWave`))
    (:`  `
      (`self.OnUpdateWave` _result)
      (set `self.SpawnAllEnemyInWave` false)
      (set `self.QuantityEnemySpawn` 0)
      (bind _returnvalue (`KismetSystemLibrary.K2_SetTimerDelegate` (delegate `SpawnEnemy`) _output_intervalspawnenemy true false 0.01))
      (set `self.Timer` _returnvalue))))

(event `SpawnEnemy`
  (bind _output_enemy (break `/Game/TestSkillbox/Blueprint/Structure/S_WaveSetting` (`|GetArrayItem` (`self.Wave`) (- (`self.CurrentWave`) 1))))
  ;[0 0 0] Создание противников
  (bind _returnvalue (`|SpawnActorFromClass` (`KismetArrayLibrary.Array_Random` (`self.EnemyClass`)) (`KismetArrayLibrary.Array_Random` (`self.PointSpawn`)) "AlwaysSpawn" "MultiplyWithRoot" null null))
  (`/Engine/EditorBlueprintResources/StandardMacros.IsValid` _returnvalue
    (:`Is Valid`
      (add `/Game/TestSkillbox/Blueprint/Character/BP_BaseCharacter.OnDeath` _returnvalue (delegate `EnemyDeath`))
      (`/Engine/EditorBlueprintResources/StandardMacros.IncrementInt` (`self.QuantityEnemySpawn`)
        (:`  `
          (`/Engine/EditorBlueprintResources/StandardMacros.IncrementInt` (`self.QuantityEnemyInLevel`)
            (:`  `
              (if (not (> _output_enemy (`self.QuantityEnemySpawn`)))
                (`KismetSystemLibrary.K2_ClearAndInvalidateTimerHandle` (`self.Timer`))
                (set `self.SpawnAllEnemyInWave` true)))))))))

(event `EnemyDeath`
  (bind (_output_enemy _output_intervalspawnenemy _output_timefornextwave) (break `/Game/TestSkillbox/Blueprint/Structure/S_WaveSetting` (`|GetArrayItem` (`self.Wave`) (- (`self.CurrentWave`) 1))))
  ;[0 0 0] Создание противников
  (bind _result (`/Engine/EditorBlueprintResources/StandardMacros.DecrementInt` (`self.QuantityEnemyInLevel`))
    (:`  `
      (if (and (== _result 0) (`self.SpawnAllEnemyInWave`))
        (if (> (+ (`self.CurrentWave`) 1) (`KismetArrayLibrary.Array_Length` (`self.Wave`)))
          (`KismetSystemLibrary.Delay` 3.0)
          (`/Game/TestSkillbox/Core/BP_TestSkillBox_GM.EndGame` (`/Game/TestSkillbox/Blueprint/DataAsset/PDA_GameplayClasses.TestSkillbox_GM` (`self.GameplayClasses`)) true)
          (else
            (`|ExecutionSequence`
              (:`then_0`
                (`KismetSystemLibrary.Delay` _output_timefornextwave)
                (`self.SpawnWave`))
              (:`then_1`
                (`KismetSystemLibrary.Delay` 2.0)
                (`UserWidget.AddToViewport` (`self.Upgrate`) 0)
                (`/Game/TestSkillbox/Core/BP_TestSkillBox_GM.SetInputMode` (`/Game/TestSkillbox/Blueprint/DataAsset/PDA_GameplayClasses.TestSkillbox_GM` (`self.GameplayClasses`)) "NewEnumerator1")))))))))

(fn `UserConstructionScript`)