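; AI enemy character that fights with a rifle and drops a random bonus when killed.
; On BeginPlay it links its health widget, spawns a rifle on its spine and enters shoot mode.
; ModeShoot plays the equip montage forward or reversed, using notifies to move the rifle between spine and hand, and toggles the GA_ModeShoot ability.
; Death ragdolls, removes the widget, flags the Blackboard, destroys the controller, then destroys weapon and self after a delay.
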(event `self.Death`
  (bind _returnvalue (`AIBlueprintHelperLibrary.GetAIController` self))
  ;[0 0 0] Смерть врага, Ragdoll, уничтожение врага и его контроллера
  (`parent.Death`)
  (`self.Ragdoll` true)
  (`|SpawnActorFromClass` (`KismetArrayLibrary.Array_Random` (`self.BonusSpawn`)) (`KismetMathLibrary.MakeTransform` (- (`self.K2_GetActorLocation`) (0.0 0.0 80.0))) "Undefined" "MultiplyWithRoot" null null)
  (`ActorComponent.K2_DestroyComponent` (`self.Widget`))
  (bind _blackboard (`AIController.Blackboard` _returnvalue)
    (:`then`
      (`BlackboardComponent.SetValueAsBool` _blackboard "Death" true))
    (:`else`
      _))
  (`self.K2_DestroyActor` _returnvalue)
  (`KismetSystemLibrary.Delay` 2.0)
  (bind _activeweapon (`self.ActiveWeapon`)
    (:`then`
      (`self.K2_DestroyActor` _activeweapon))
    (:`else`
      _))
  (`self.K2_DestroyActor`))

(event `self.ReceiveBeginPlay`
  (bind _spine (`self.Spine`))
  ;[0 0 0] Запись себя в виджет здоровья, создание оружия и крепление к себе
  (`parent.ReceiveBeginPlay`)
  (bind _aswbp_health (cast `/Game/TestSkillbox/Widget/WBP_Health` (`WidgetComponent.GetWidget` (`self.Widget`))))
  (set `/Game/TestSkillbox/Widget/WBP_Health.Owner` self _aswbp_health)
  (bind _returnvalue (`|SpawnActorFromClass` "/Game/TestSkillbox/Blueprint/Environment/Weapon/BP_Rifle.BP_Rifle_C" (`KismetMathLibrary.MakeTransform` (0.0 0.0 0.0)) "Undefined" "MultiplyWithRoot" null 5000 self null))
  (bind _output_get (set `self.ActiveWeapon` _returnvalue))
  (`self.K2_AttachToComponent` _output_get _spine "None" "KeepRelative" "KeepRelative" "KeepRelative" true)
  (`SceneComponent.K2_SetRelativeTransform` _spine (`KismetMathLibrary.MakeTransform` (0.0 0.0 0.0)) false false)
  (`KismetSystemLibrary.Delay` 0.2)
  (`self.ModeShoot` true))

(event `ModeShoot`
  (params (Aim :type Boolean))
  (bind _hand (`self.Hand`))
  (bind _spine (`self.Spine`))
  ;[0 0 0] Режим стрельбы
  (if Aim
    (if (not (`NavMovementComponent.IsFalling` (`self.CharacterMovement`)))
      (`|ExecutionSequence`
        (:`then_0`
          (goto _label_2 :!via `Open`))
        (:`then_1`
          (`|PlayMontage` (`self.Mesh`) "/Game/TestSkillbox/Animation/MannyASP/AM_Equip_Rifle.AM_Equip_Rifle"
            (:`OnBlendOut`
              (`self.ActiveAbility` true "/Game/TestSkillbox/Blueprint/AbilitySystem/GA_ModeShoot.GA_ModeShoot_C" :!label _label))
            (:`OnInterrupted`
              (goto _label))
            (:`OnNotifyBegin`
              (`/Engine/EditorBlueprintResources/StandardMacros.Gate` true :!label _label_2
                (:`Exit`
                  (`|ExecutionSequence`
                    (:`then_0`
                      (`self.K2_AttachToComponent` (`self.ActiveWeapon`) _hand "None" "KeepRelative" "KeepRelative" "KeepRelative" true)
                      (`SceneComponent.K2_SetRelativeTransform` _hand (`KismetMathLibrary.MakeTransform` (0.0 0.0 0.0)) false false))
                    (:`then_1`
                      (goto _label_3 :!via `Reset`))))))))))
    (else
      (`|ExecutionSequence`
        (:`then_0`
          (goto _label_2 :!via `Close`))
        (:`then_1`
          (`|PlayMontage` (`self.Mesh`) "/Game/TestSkillbox/Animation/MannyASP/AM_Equip_Rifle.AM_Equip_Rifle" -1.0 1.13
            (:`then`
              (`self.ActiveAbility` false "/Game/TestSkillbox/Blueprint/AbilitySystem/GA_ModeShoot.GA_ModeShoot_C"))
            (:`OnNotifyBegin`
              (`/Engine/EditorBlueprintResources/StandardMacros.DoOnce` true :!label _label_3
                (:`Completed`
                  (`KismetSystemLibrary.Delay` 0.5)
                  (`self.K2_AttachToComponent` (`self.ActiveWeapon`) _spine "None" "KeepRelative" "KeepRelative" "KeepRelative" true)
                  (`SceneComponent.K2_SetRelativeTransform` _spine (`KismetMathLibrary.MakeTransform` (0.0 0.0 0.0)) false false))))))))))

(fn `UserConstructionScript`
  (`parent.UserConstructionScript`))