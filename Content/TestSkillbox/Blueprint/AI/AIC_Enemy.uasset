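; AI controller for BP_Enemy that runs the BT_Enemy behavior tree shortly after possession.
; Perception updates write player sight, last stimulus location and visibility of the blackboard Target into the blackboard, setting or clearing focus.
; The PlayerAttack handler for damage taken records the damage causer's location and an Attacked flag, dropping focus if the causer is not the focused actor.
; Actors of the enemy's own class are ignored.
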(event `self.ReceivePossess`
  (params (PossessedPawn :type "Pawn Object Reference"))
  ;[0 0 0] Запуск дерева поведения
  (bind _asbp_enemy (cast `/Game/TestSkillbox/Blueprint/AI/Enemy/BP_Enemy` PossessedPawn))
  (bind _output_get (set `self.Enemy` _asbp_enemy))
  (add `self.OnTakeAnyDamage` _output_get (`|CreateDelegate` :!event `PlayerAttack`))
  (`KismetSystemLibrary.Delay` 1.0)
  (`self.RunBehaviorTree` "/Game/TestSkillbox/Blueprint/AI/BT_Enemy.BT_Enemy"))

(event `self.AIPerception.OnTargetPerceptionUpdated`
  (params (Actor :type "Actor Object Reference") (Stimulus :type "AIStimulus Structure"))
  (bind ((`StimulusLocation` _stimuluslocation) (`bSuccessfullySensed` _bsuccessfullysensed)) (break `AIStimulus` Stimulus))
  (bind _blackboard (`self.Blackboard`))
  (bind _blackboard_2 (`self.Blackboard`))
  ;[0 0 0] Запись данных обнаружения в дерево поведения
  (set `self.Actor` Actor)
  (`self.Blackboard`
    (:`then`
      (if (!= (`GameplayStatics.GetObjectClass` Actor) (`GameplayStatics.GetObjectClass` (`self.Enemy`)))
        (bind _asbp_test_skillbox_p (cast `/Game/TestSkillbox/Core/BP_TestSkillbox_P` (`self.Actor`))
          (:`then`
            (if _bsuccessfullysensed
              (`self.K2_SetFocus` _asbp_test_skillbox_p)
              (`BlackboardComponent.SetValueAsBool` _blackboard "PlayerSee" true)
              (`BlackboardComponent.SetValueAsVector` _blackboard "PlayerLocation" _stimuluslocation)
              (else
                (`self.K2_ClearFocus`)
                (`BlackboardComponent.ClearValue` _blackboard "PlayerSee")
                (`BlackboardComponent.SetValueAsVector` _blackboard "PlayerLocation" _stimuluslocation))))
          (:`CastFailed`
            (if (== (`self.Actor`) (`BlackboardComponent.GetValueAsObject` (`self.Blackboard`) "Target"))
              (if _bsuccessfullysensed
                (`BlackboardComponent.SetValueAsBool` _blackboard_2 "TargetSee" true)
                (`self.K2_SetFocus` (`self.Actor`))
                (else
                  (`BlackboardComponent.ClearValue` _blackboard_2 "TargetSee"))))))))
    (:`else`)))

(event `PlayerAttack` :!signature `self.OnTakeAnyDamage`
  (params (DamagedActor :type "Actor Object Reference") (Damage :type "Float (single-precision)") (DamageType :type "DamageType Object Reference") (InstigatedBy :type "Controller Object Reference") (DamageCauser :type "Actor Object Reference"))
  ;[0 0 0] Запись информации о атаке игрока
  (`/Engine/EditorBlueprintResources/StandardMacros.IsValid` DamageCauser
    (:`Is Valid`
      (if (!= (`GameplayStatics.GetObjectClass` DamageCauser) (`GameplayStatics.GetObjectClass` (`self.Enemy`)))
        (bind _blackboard (`self.Blackboard`)
          (:`then`
            (`BlackboardComponent.SetValueAsVector` _blackboard "PlayerLocation" (`self.K2_GetActorLocation` DamageCauser))
            (`BlackboardComponent.SetValueAsBool` _blackboard "Attacked" true)
            (if (!= DamageCauser (`self.GetFocusActor`))
              (`self.K2_ClearFocus`)))
          (:`else`))))))

(fn `UserConstructionScript`)