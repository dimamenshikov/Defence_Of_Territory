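; BP_BaseCharacter is a character Blueprint providing Gameplay Ability System abilities, death handling and ragdoll toggling.
; BeginPlay grants each listed ability with its array index as InputID, which ActiveAbility uses to press or release it.
; Zero health triggers a one-time death with sound, blood, GE_Death and an OnDeath call.
; Ragdoll switches mesh physics and capsule collision, while construction attaches Hand and Spine points to skeleton sockets.
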(event `self.ReceiveBeginPlay`
  ;[0 0 0] Добавление способностей к персонажу
  (for (_array_element _array_index) (`self.Abilities`)
    (`AbilitySystemComponent.K2_GiveAbility` (`self.AbilitySystem`) _array_element 0 _array_index)))

(event `Ragdoll`
  (params (bRagdoll :type Boolean :default true))
  (bind _mesh (`self.Mesh`))
  (bind _capsulecomponent (`self.CapsuleComponent`))
  ;[0 0 0] Включение/отключение ragdoll
  (bind _output_get (set `self.bDeath` bRagdoll))
  (if _output_get
    (`PrimitiveComponent.SetSimulatePhysics` _mesh true)
    (`PrimitiveComponent.SetCollisionEnabled` _capsulecomponent "NoCollision")
    (else
      (`PrimitiveComponent.SetSimulatePhysics` _mesh false)
      (`SceneComponent.K2_SetRelativeTransform` (`self.Mesh`) (`KismetMathLibrary.MakeTransform` (0.0 0.0 -90.0) (struct :`Yaw` -90.0)) false false)
      (`PrimitiveComponent.SetCollisionEnabled` _capsulecomponent "QueryAndPhysics"))))

(event `/Game/TestSkillbox/Blueprint/Interface/BPI_Damage.Damage`
  (params (Damage :type "Float (double-precision)") (Health :type "Float (double-precision)"))
  (bind _returnvalue (`self.K2_GetActorLocation`))
  (bind (_gamesetting_sound _gamesetting_music _gamesetting_audio) (break `/Game/TestSkillbox/Blueprint/Structure/S_GameSetting` (`/Game/TestSkillbox/Core/BP_TestSkillbox_GI.GameSetting` (`/Game/TestSkillbox/Blueprint/DataAsset/PDA_GameplayClasses.TestSkillbox_GI` (`self.GameplayClasses`)))))
  ;[0 0 0] Смерть персонажа
  (if (== Health 0.0)
    (`/Engine/EditorBlueprintResources/StandardMacros.DoOnce` false
      (:`Completed`
        (`GameplayStatics.PlaySoundAtLocation` "/Game/TestSkillbox/Assets/Audio/A_Death.A_Death" _returnvalue (struct) (* _gamesetting_sound _gamesetting_audio) 1.0 0.0 null null null null)
        (`GameplayStatics.SpawnEmitterAtLocation` "/Game/TestSkillbox/Assets/Effect/Blood/P_Blood.P_Blood" _returnvalue (struct) (3.0 3.0 3.0))
        (`AbilitySystemComponent.BP_ApplyGameplayEffectToSelf` :`self` (`self.AbilitySystem`) :`GameplayEffectClass` "/Game/TestSkillbox/Blueprint/AbilitySystem/Effect/GE_Death.GE_Death_C")
        (`self.OnDeath`)
        (`self.Death`)))))

(event `Death`
  ;[0 0 0] Смерть персонажа
  (set `self.bDeath` true))

(fn `ActiveAbility`
  (params (Activate :type Boolean) (ActiveAbility :type "/Game/TestSkillbox/Blueprint/AbilitySystem/GA_BaseAbilty Class Reference"))
  (bind _abilitysystem (`self.AbilitySystem`))
  (bind _returnvalue (`KismetArrayLibrary.Array_Find` (`self.Abilities`) ActiveAbility))
  ;[0 0 0] Активация/деактивация способности
  (if Activate
    (`AbilitySystemComponent.PressInputID` _abilitysystem _returnvalue)
    (else
      (`AbilitySystemComponent.ReleaseInputID` _abilitysystem _returnvalue))))

(fn `UserConstructionScript`
  ;[0 0 0] Крепление точек к скелету
  (`SceneComponent.K2_AttachToComponent` (`self.Hand`) (`self.Mesh`) (`self.SocketHand`) "KeepRelative" "KeepRelative" "KeepRelative" true)
  (`SceneComponent.K2_AttachToComponent` (`self.Spine`) (`self.Mesh`) (`self.SocketSpine`) "KeepRelative" "KeepRelative" "KeepRelative" true))